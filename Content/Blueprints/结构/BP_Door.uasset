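; BP_Door is an automatic door that moves aside when a Character enters its Box trigger and returns when one leaves.
; Overlap begin plays a timeline and overlap end reverses it from the end.
; Each update adds the timeline's X and Y track values to SimpleDoor as world offsets, negated when reversing, so movement accumulates per tick rather than interpolating between set positions.
; A rotating-door node is left unconnected.
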(event `self.Box.OnComponentBeginOverlap`
  (params (OverlappedComponent :type "PrimitiveComponent Object Reference") (OtherActor :type "Actor Object Reference") (OtherComp :type "PrimitiveComponent Object Reference") (OtherBodyIndex :type Integer) (bFromSweep :type Boolean) (SweepResult :type "HitResult Structure (by ref)"))
  (bind _simpledoor (`self.SimpleDoor`))
  (cast `Character` OtherActor)
  (bind (_direction `_y轴运动` `_x轴运动`) (`Timeline|时间轴_0` :!label _label)
    (:`Update`
      (switch `ETimelineDirection` _direction
        (:`Forward`
          (`SceneComponent.K2_AddWorldOffset` _simpledoor (`KismetMathLibrary.MakeVector` 0.0 `_y轴运动`) false false)
          (`SceneComponent.K2_AddWorldOffset` _simpledoor (`KismetMathLibrary.MakeVector` `_x轴运动`) false false))
        (:`Backward`
          (`SceneComponent.K2_AddWorldOffset` _simpledoor (`KismetMathLibrary.MakeVector` 0.0 (* `_y轴运动` -1.0)) false false)
          (`SceneComponent.K2_AddWorldOffset` _simpledoor (`KismetMathLibrary.MakeVector` (* `_x轴运动` -1.0)) false false))))))

(event `self.Box.OnComponentEndOverlap`
  (params (OverlappedComponent :type "PrimitiveComponent Object Reference") (OtherActor :type "Actor Object Reference") (OtherComp :type "PrimitiveComponent Object Reference") (OtherBodyIndex :type Integer))
  (cast `Character` OtherActor)
  (goto _label :!via `ReverseFromEnd`))

(fn `UserConstructionScript`)