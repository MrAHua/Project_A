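; Tifa Lockhart character Blueprint with Shift sprinting and two-step melee combos: punches on left mouse, kicks on right.
; Both attacks share one montage path, choosing a section by a common ComboIndex and freezing movement during playback.
; Blend-out restores walk speed, advances the index and starts a short timer that resets the combo.
; BeginPlay applies GE_Damage to itself through the Ability System Component.
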(event `self.ReceiveBeginPlay`
  (`AbilitySystemComponent.BP_ApplyGameplayEffectToSelf` :`self` (`self.AbilitySystemComponent`) :`GameplayEffectClass` "/Game/Blueprints/Abilities/GameEffects/GE_Damage.GE_Damage_C"))

(event `Key|LeftShift`
  (params (Key :type "Key Structure"))
  (bind _charactermovement (`self.CharacterMovement`))
  (:`Pressed`
    (set `CharacterMovementComponent.MaxWalkSpeed` 500.0 _charactermovement))
  (:`Released`
    (set `CharacterMovementComponent.MaxWalkSpeed` 200.0 _charactermovement)))

(event `Key|LeftMouseButton`
  (params (Key :type "Key Structure"))
  (bind _timerhandle (`self.TimerHandle`))
  (bind _charactermovement (`self.CharacterMovement`))
  (:`Pressed`
    (`KismetArrayLibrary.Array_Clear` (`self.ComboSections`))
    (set `self.ComboSections` (`|MakeArray` "Light_Punch" "Heavy_Punch" :!type "Name"))
    (set `self.Montage to Play` "/Game/Characters/Tifa/AnimationTest/Montage/PunchCombat.PunchCombat")
    (if (`KismetSystemLibrary.K2_IsValidTimerHandle` _timerhandle) :!label _label
      (`KismetSystemLibrary.K2_ClearAndInvalidateTimerHandle` _timerhandle))
    (if (not (`self.IsPlayingMontage`))
      (`|PlayMontage` (`self.Mesh`) (`self.Montage to Play`) 1.5 0.0 (`|GetArrayItem` (`self.ComboSections`) (`self.ComboIndex`))
        (:`then`
          (if (`self.IsPlayingMontage`)
            (set `CharacterMovementComponent.MaxWalkSpeed` 0.0 _charactermovement)))
        (:`OnBlendOut`
          (set `CharacterMovementComponent.MaxWalkSpeed` 200.0 _charactermovement)
          (if (< (`self.ComboIndex`) (- (`KismetArrayLibrary.Array_Length` (`self.ComboSections`)) 1))
            (`/Engine/EditorBlueprintResources/StandardMacros.IncrementInt` (`self.ComboIndex`)
              (:`  `
                _)))
          (bind _returnvalue (`KismetSystemLibrary.K2_SetTimerDelegate` (delegate `Reset Combo Index`) 0.1))
          (bind _output_get (set `self.TimerHandle` _returnvalue)))))))

(event `Key|RightMouseButton`
  (params (Key :type "Key Structure"))
  (:`Pressed`
    (`KismetArrayLibrary.Array_Clear` (`self.ComboSections`))
    (set `self.ComboSections` (`|MakeArray` "Light_Kick" "Kick_Round" :!type "Name"))
    (set `self.Montage to Play` "/Game/Characters/Tifa/AnimationTest/Montage/KickCombat.KickCombat")
    (goto _label)))

(event `Reset Combo Index`
  (set `self.ComboIndex` 0)
  (`KismetSystemLibrary.K2_ClearAndInvalidateTimerHandle` (stale `Key|LeftMouseButton` _output_get)))

(fn `UserConstructionScript`)