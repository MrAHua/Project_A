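; BP_Fire is an interactive fire hazard that damages Tifa over time while she stands in its box.
; Box overlap stores the entering actor and starts a looping one-second timer, which any end overlap clears.
; Each tick casts that actor to BP_Tifa_Lockhart and applies GE_Damage through her Ability System Component.
; A HitSelect event hides the actor in game, without clearing the timer or disabling collision.
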(event `self.Box.OnComponentBeginOverlap`
  (params (OverlappedComponent :type "PrimitiveComponent Object Reference") (OtherActor :type "Actor Object Reference") (OtherComp :type "PrimitiveComponent Object Reference") (OtherBodyIndex :type Integer) (bFromSweep :type Boolean) (SweepResult :type "HitResult Structure (by ref)"))
  (set `self.Other Actor` OtherActor)
  (bind _returnvalue (`KismetSystemLibrary.K2_SetTimerDelegate` (delegate `DamageTick`) 1.0 true))
  (set `self.TimerHandle` _returnvalue))

(event `DamageTick`
  (bind _asbp_tifa_lockhart (cast `/Game/Blueprints/Characters/BP_Tifa_Lockhart` (`self.Other Actor`)))
  (`AbilitySystemComponent.BP_ApplyGameplayEffectToSelf` :`self` (`AbilitySystemBlueprintLibrary.GetAbilitySystemComponent` _asbp_tifa_lockhart) :`GameplayEffectClass` "/Game/Blueprints/Abilities/GameEffects/GE_Damage.GE_Damage_C"))

(event `self.Box.OnComponentEndOverlap`
  (params (OverlappedComponent :type "PrimitiveComponent Object Reference") (OtherActor :type "Actor Object Reference") (OtherComp :type "PrimitiveComponent Object Reference") (OtherBodyIndex :type Integer))
  (`KismetSystemLibrary.K2_ClearAndInvalidateTimerHandle` (`self.TimerHandle`)))

(event `/Game/Interfaces/BPI_HitSelect.HitSelect`
  (`self.SetActorHiddenInGame` self true))

(fn `UserConstructionScript`)