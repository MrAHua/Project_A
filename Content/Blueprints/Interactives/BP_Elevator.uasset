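; BP_Elevator is an elevator actor that moves to a requested floor's target location.
; On BeginPlay it records its location and gathers all BP_TargetFloor actors in the level.
; GetTargetFloorWorkdLocation matches a FloorIndex against those actors, stores the target location and calls ElevatorRunning.
; The ElevatorMove timeline lerps SceneComponent's world position to the target without sweep, then saves the actor location as the next start point.
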(event `self.ReceiveBeginPlay`
  (set `self.CurrentElevatorLocation` (`self.K2_GetActorLocation`))
  (bind _outactors (`GameplayStatics.GetAllActorsOfClass` "/Game/Blueprints/Interactives/BP_TargetFloor.BP_TargetFloor_C"))
  (bind _output_get (set `self.TargetFloorLocations` _outactors))
  (`KismetSystemLibrary.PrintString` (`KismetStringLibrary.Concat_StrStr` "找到  " (`KismetStringLibrary.Conv_IntToString` (`KismetArrayLibrary.Array_Length` _output_get)) "  个楼层目标")))

(event `GetTargetFloorWorkdLocation`
  (params (FloorIndex :type Integer))
  (for _array_element (`self.TargetFloorLocations`)
    (if (== (`/Game/Blueprints/Interactives/BP_TargetFloor.FloorIndex` _array_element) FloorIndex)
      (bind _output_get (set `self.TargetFloorLocation` (`/Game/Blueprints/Interactives/BP_TargetFloor.CurrentTargetFloorLocation` _array_element)))
      (`KismetSystemLibrary.PrintString` (`KismetStringLibrary.Conv_VectorToString` _output_get))
      (`self.ElevatorRunning`))))

(event `ElevatorRunning`
  (bind (_direction `_新建轨道_1`) (`Timeline|ElevatorMove` :!via `PlayFromStart`)
    (:`Update`
      (`SceneComponent.K2_SetWorldLocation` (`self.SceneComponent`) (`KismetMathLibrary.VLerp` (`self.CurrentElevatorLocation`) (`self.TargetFloorLocation`) `_新建轨道_1`) false false))
    (:`Finished`
      (set `self.CurrentElevatorLocation` (`self.K2_GetActorLocation`)))))

(fn `UserConstructionScript`)