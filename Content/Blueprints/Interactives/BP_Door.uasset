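; BP_Door is an interactive door that slides along a spline when a Character enters its collision box.
; On overlap it caches the door's world location, then a timeline offsets it by local spline position scaled by spline length, with zeroed rotation.
; Leaving the box reverses the timeline from its end.
; The base location is re-cached on every entry, even if the door is mid-motion.
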(event `self.CollisionBox.OnComponentBeginOverlap`
  (params (OverlappedComponent :type "PrimitiveComponent Object Reference") (OtherActor :type "Actor Object Reference") (OtherComp :type "PrimitiveComponent Object Reference") (OtherBodyIndex :type Integer) (bFromSweep :type Boolean) (SweepResult :type "HitResult Structure (by ref)"))
  (bind _spline (`self.Spline`))
  (bind _simpledoor (`self.SimpleDoor`))
  (cast `Character` OtherActor)
  (set `self.CurrentLocation` (`SceneComponent.K2_GetComponentLocation` _simpledoor))
  (bind (_direction `_y轴运动`) (`Timeline|时间轴_0` :!label _label)
    (:`Update`
      (`SceneComponent.K2_SetWorldTransform` (`self.SimpleDoor`) (`KismetMathLibrary.MakeTransform` (+ (`self.CurrentLocation`) (`SplineComponent.GetLocationAtDistanceAlongSpline` _spline (* `_y轴运动` (`SplineComponent.GetSplineLength` _spline)) "Local")) (struct) (`SceneComponent.K2_GetComponentScale` _simpledoor)) false false))))

(event `self.CollisionBox.OnComponentEndOverlap`
  (params (OverlappedComponent :type "PrimitiveComponent Object Reference") (OtherActor :type "Actor Object Reference") (OtherComp :type "PrimitiveComponent Object Reference") (OtherBodyIndex :type Integer))
  (cast `Character` OtherActor)
  (goto _label :!via `ReverseFromEnd`))

(fn `UserConstructionScript`)