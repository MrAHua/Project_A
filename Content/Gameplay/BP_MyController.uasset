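; BP_MyController handles left-click selection of actors in the world, judging by its name as a controller.
; A click deprojects the mouse position into a debug-drawn Visibility line trace.
; It then gets all actors of the hit actor's class and calls HitSelectMessage on the first, which is not necessarily the one clicked.
; A BP_Spline cast and a tag lookup are left unconnected.
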(event `self.ReceiveBeginPlay`)

(event `Key|LeftMouseButton`
  (params (Key :type "Key Structure"))
  (bind (_worldlocation _worlddirection) (`self.DeprojectMousePositionToWorld`))
  (:`Pressed`
    (bind _outhit (`KismetSystemLibrary.LineTraceSingle` :`Start` _worldlocation :`End` (+ _worldlocation (* _worlddirection 9999.0)) :`TraceChannel` "TraceTypeQuery1" :`DrawDebugType` "ForDuration"))
    (bind _output_get (set `self.Out Hit` _outhit))
    (bind _outactors (`GameplayStatics.GetAllActorsOfClass` (`GameplayStatics.GetObjectClass` (`.HitActor` (`GameplayStatics.BreakHitResult` _output_get)))))
    (if (`KismetArrayLibrary.Array_IsValidIndex` _outactors)
      (message `/Game/Interfaces/BPI_HitSelect.HitSelect` (`|GetArrayItem` _outactors)))))

(fn `UserConstructionScript`)